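; BP_Role is a role actor that shows its San (likely sanity) value through an overhead WCHP health display.
; The construction script places WCHP 150 units above the actor and starts it full.
; Every Tick sets the display's CurHP to the ratio of CurrentSanValue to SanValue, with no zero check on the divisor.
; BeginPlay is empty and the overlap event is disabled.
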(event `self.ReceiveBeginPlay`)

(event `self.ReceiveTick`
  (params (DeltaSeconds :type "Float (single-precision)"))
  (set `/Game/UI/WC_HP.CurHP` (/ (`self.CurrentSanValue`) (`self.SanValue`)) (`self.WC_HP`)))

(fn `UserConstructionScript`
  (bind _wc_hp (`self.WC_HP`))
  (`SceneComponent.K2_SetWorldLocation` _wc_hp (+ (`self.K2_GetActorLocation`) (0.0 0.0 150.0)) false false)
  (set `/Game/UI/WC_HP.CurHP` 1.0 _wc_hp))