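; BP_Camera is a camera Blueprint that follows the CurrentRole actor.
; On BeginPlay it stores a relative transform computed between its own transform and that of CurrentRole.
; Each Tick it composes that offset with the role's current transform and sets its own transform, without sweep or smoothing, acting like a rigid attachment without actually attaching.
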(event `self.ReceiveBeginPlay`
  (set `self.RelativeTransform` (`KismetMathLibrary.ConvertTransformToRelative` (`self.GetTransform` (`self.CurrentRole`)) (`self.GetTransform` self))))

(event `self.ReceiveTick`
  (params (DeltaSeconds :type "Float (single-precision)"))
  (`self.K2_SetActorTransform` self (`KismetMathLibrary.ComposeTransforms` (`self.RelativeTransform`) (`self.GetTransform` (`self.CurrentRole`))) false false))

(fn `UserConstructionScript`)