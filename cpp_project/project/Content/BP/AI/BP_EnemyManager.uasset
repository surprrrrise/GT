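; BP_EnemyManager is a manager Blueprint that tracks the enemies in the level and cleans up those flagged for removal.
; On BeginPlay it fills EnemyList with every BP_enemy actor found at that moment.
; Each Tick it polls the list, destroying any non-null enemy whose CanBeRemove flag is set and removing its index while still iterating the same array.
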(event `self.ReceiveBeginPlay`
  (bind _outactors (`GameplayStatics.GetAllActorsOfClass` "/Game/BP/AI/BP_enemy.BP_enemy_C"))
  (set `self.EnemyList` _outactors))

(event `self.ReceiveTick`
  (params (DeltaSeconds :type "Float (single-precision)"))
  (bind _enemylist (`self.EnemyList`))
  (for (_array_element _array_index) _enemylist
    (if (not (== _array_element null))
      (if (`/Game/BP/AI/BP_enemy.CanBeRemove` _array_element)
        (`self.K2_DestroyActor` _array_element)
        (`KismetArrayLibrary.Array_Remove` _enemylist _array_index)))))

(fn `UserConstructionScript`)