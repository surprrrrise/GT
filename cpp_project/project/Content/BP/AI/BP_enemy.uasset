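; Enemy actor that tracks hit points, shows them on an overhead health bar (WCHP) and flags its own death.
; The construction script places the bar above the actor, turns it once toward the BP_Camera actor and stores starting HP as TotlaHP.
; Tick feeds the HP ratio to the bar and sets CanBeRemove when HP reaches zero, without destroying the actor here.
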(event `self.ReceiveTick`
  (params (DeltaSeconds :type "Float (single-precision)"))
  (bind _hp (`self.HP`))
  (set `/Game/UI/WC_HP.CurHP` (/ (`KismetMathLibrary.Conv_IntToDouble` _hp) (`KismetMathLibrary.Conv_IntToDouble` (`self.TotlaHP`))) (`self.WC_HP`))
  ;[1 1 1] 死亡
  (if (<= _hp 0)
    (set `self.CanBeRemove` true)))

(fn `UserConstructionScript`
  (bind _returnvalue (`GameplayStatics.GetActorOfClass` "/Game/BP/BP_Camera.BP_Camera_C"))
  (set `self.Camera` _returnvalue)
  (`SceneComponent.K2_SetWorldLocation` (`self.WC_HP`) (+ (`self.K2_GetActorLocation`) (0.0 0.0 150.0)) false false)
  (`SceneComponent.K2_SetWorldRotation` (`self.WC_HP`) (`KismetMathLibrary.FindLookAtRotation` (`SceneComponent.K2_GetComponentLocation` (`self.WC_HP`)) (`self.K2_GetActorLocation` (`self.Camera`))) false false)
  (set `/Game/UI/WC_HP.CurHP` 1.0 (`self.WC_HP`))
  (set `self.TotlaHP` (`self.HP`)))