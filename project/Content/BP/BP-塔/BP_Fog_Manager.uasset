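; Fog manager actor that temporarily clears fog on the level's BP塔基Blank grid tiles.
; BeginPlay gathers the tiles, and SetEnable changes a given tile's status and starts its AliveTime countdown in parallel arrays.
; Each Tick decrements timers by one, so lifetime is frame-based, resets expired statuses, then calls SetFog on every tile.
; Init appends 64 default entries in both construction script and BeginPlay without clearing.
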(event `self.ReceiveBeginPlay`
  (bind _outactors (`GameplayStatics.GetAllActorsOfClass` "/Game/BP/BP-塔/BP-塔基Blank.BP-塔基Blank_C"))
  (set `self.GridArray` _outactors)
  (`self.Init`))

(event `self.ReceiveTick`
  (params (DeltaSeconds :type "Float (single-precision)"))
  (`self.UpdateLifetime`)
  (`self.UpdateGrid`))

(fn `Init`
  ;[0.09797 0.0904 1] 初始化状态数组
  (for _ (range 64)
    (`KismetArrayLibrary.Array_Add` (`self.GridStatusArray`) "NewEnumerator0")
    (`KismetArrayLibrary.Array_Add` (`self.GridTimeArray`))))

(fn `SetEnable`
  (params (Target :type "/Game/BP/BP-塔/BP-塔基Blank Object Reference"))
  (bind _returnvalue (`KismetArrayLibrary.Array_Find` (`self.GridArray`) Target))
  (if (>= _returnvalue 0)
    (`KismetArrayLibrary.Array_Set` (`self.GridStatusArray`) _returnvalue "NewEnumerator1")
    (`KismetArrayLibrary.Array_Set` (`self.GridTimeArray`) _returnvalue (`self.AliveTime`))))

(fn `UpdateGrid`
  (locals (temp :type "/Game/BP/BP-塔/E_Grid_Status Enum" :default "NewEnumerator0"))
  (for (_array_element _array_index) (`self.GridArray`)
    (if (`|EnumEquality` (`|GetArrayItem` (`self.GridStatusArray`) _array_index) (`local.temp`))
      (`/Game/BP/BP-塔/BP-塔基Blank.SetFog` _array_element false)
      (else
        (`/Game/BP/BP-塔/BP-塔基Blank.SetFog` _array_element true)))))

(fn `UpdateLifetime`
  (for (_array_element _array_index) (`self.GridTimeArray`)
    (if (> _array_element 0)
      (bind _returnvalue (- _array_element 1))
      (`KismetArrayLibrary.Array_Set` (`self.GridTimeArray`) _array_index _returnvalue)
      (if (<= _returnvalue 0)
        (`KismetArrayLibrary.Array_Set` (`self.GridStatusArray`) _array_index "NewEnumerator0")))))

(fn `UserConstructionScript`
  (`self.Init`))